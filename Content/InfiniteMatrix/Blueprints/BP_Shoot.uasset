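; BP_Shoot is a player projectile that flies along world X and destroys any BP_Monster it overlaps.
; Every tick it looks up BP_Player, sets the projectile movement InitialSpeed slightly above the player's ForwardSpeed, and uses that to offset itself manually.
; On a monster hit it calls the player's TraverseTriggerZone, refreshes the HealthWidget score text and prints a debug message.
; The projectile does not destroy itself on impact.
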(event `self.ReceiveTick`
  (params (DeltaSeconds :type "Float (single-precision)"))
  (bind _outactors (`GameplayStatics.GetAllActorsOfClass` "/Game/InfiniteMatrix/Blueprints/BP_Player.BP_Player_C"))
  (bind _output_get (set `ProjectileMovementComponent.InitialSpeed` (* (`/Game/InfiniteMatrix/Blueprints/BP_Player.ForwardSpeed` (`|GetArrayItem` _outactors)) 1.2) (`self.ProjectileMovement`)))
  (`self.K2_AddActorWorldOffset` (`KismetMathLibrary.MakeVector` (* DeltaSeconds _output_get))))

(event `self.projectile.OnComponentBeginOverlap`
  (params (OverlappedComponent :type "PrimitiveComponent Object Reference") (OtherActor :type "Actor Object Reference") (OtherComp :type "PrimitiveComponent Object Reference") (OtherBodyIndex :type Integer) (bFromSweep :type Boolean) (SweepResult :type "HitResult Structure (by ref)"))
  (bind _asbp_monster (cast `/Game/InfiniteMatrix/Blueprints/BP_Monster` OtherActor))
  (bind _outactors (`GameplayStatics.GetAllActorsOfClass` "/Game/InfiniteMatrix/Blueprints/BP_Player.BP_Player_C"))
  (bind _output (`|GetArrayItem` _outactors))
  (`/Game/InfiniteMatrix/Blueprints/BP_Player.traverseTriggerZone` _output)
  (`/Game/InfiniteMatrix/UI/WBT_HealthSystem.updateScoreText` (`/Game/InfiniteMatrix/Blueprints/BP_Player.HealthWidget` _output))
  (`self.K2_DestroyActor` _asbp_monster)
  (`KismetSystemLibrary.PrintString` "Hit"))

(fn `UserConstructionScript`)